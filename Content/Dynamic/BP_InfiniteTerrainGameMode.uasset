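; Game mode for an infinite terrain level that spawns the initial chain of tiles and tracks the score.
; On BeginPlay it populates a nav mesh bounds volume pool, then spawns several BP_Tile actors in sequence.
; Each tile receives the shared pool and returns an attach location, which becomes the spawn transform for the next tile.
; NewTileConquered increments the score, which GetScore exposes.
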(event `self.ReceiveBeginPlay`
  (`self.PopulateBoundsPool`)
  (for _ (range 4)
    (`self.Spawn Tile`)))

(fn `GetScore`
  (returns (NewParam :type Integer))
  (return (`self.Score`)))

(fn `NewTileConquered`
  (`/Engine/EditorBlueprintResources/StandardMacros.IncrementInt` (`self.Score`)))

(fn `Spawn Tile`
  (bind _returnvalue (`|SpawnActorFromClass` "/Game/Dynamic/Terrain/BP_Tile.BP_Tile_C" (`self.SpawnTransform`) "Undefined" "OverrideRootScale" null null))
  (`Tile.SetPool` _returnvalue (`self.NavMeshBoundsVolumePool`))
  (bind _attachtransform (`/Game/Dynamic/Terrain/BP_Tile.GetAttachLocation` _returnvalue))
  (set `self.SpawnTransform` _attachtransform))

(fn `UserConstructionScript`)